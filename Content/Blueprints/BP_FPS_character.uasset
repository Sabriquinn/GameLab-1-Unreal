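; First-person player character Blueprint that handles walking, looking, jumping and running.
; On BeginPlay it adds the IMC_scifimap Enhanced Input mapping context to the first player controller's subsystem.
; Input actions drive movement along the actor's forward and right vectors, plus controller yaw and negated pitch for mouse look.
; Holding Run doubles the max walk speed until release.
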(event `self.ReceiveBeginPlay`
  ;[0.08209 0.5758 1] Movement
  (`EnhancedInputSubsystemInterface.AddMappingContext` (pcsubsystem `EnhancedInputLocalPlayerSubsystem` (`GameplayStatics.GetPlayerController` 0)) "/Game/Inputs/IMC_scifimap.IMC_scifimap" 0 (struct)))

(event `EnhancedInput|/Game/Inputs/WASD_movement`
  (params (ActionValue :type "Vector2D Structure") (ElapsedSeconds :type "Float (double-precision)") (TriggeredSeconds :type "Float (double-precision)") (InputAction :type "InputAction Object Reference" :default "/Game/Inputs/WASD_movement.WASD_movement"))
  ;[0.08209 0.5758 1] Movement
  (:`Triggered`
    (`self.AddMovementInput` (`self.GetActorForwardVector`) ActionValue_X)
    (`self.AddMovementInput` (`self.GetActorRightVector`) ActionValue_Y)))

(event `EnhancedInput|/Game/Inputs/Mouse_movement`
  (params (ActionValue :type "Vector2D Structure") (ElapsedSeconds :type "Float (double-precision)") (TriggeredSeconds :type "Float (double-precision)") (InputAction :type "InputAction Object Reference" :default "/Game/Inputs/Mouse_movement.Mouse_movement"))
  ;[0.08209 0.5758 1] Movement
  (:`Triggered`
    (`self.AddControllerYawInput` ActionValue_X)
    (`self.AddControllerPitchInput` (* ActionValue_Y -1.0))))

(event `EnhancedInput|/Game/Inputs/Jump`
  (params (ActionValue :type Boolean) (ElapsedSeconds :type "Float (double-precision)") (TriggeredSeconds :type "Float (double-precision)") (InputAction :type "InputAction Object Reference" :default "/Game/Inputs/Jump.Jump"))
  ;[0.08209 0.5758 1] Movement
  (:`Started`
    (`self.Jump`)))

(event `EnhancedInput|/Game/Inputs/Run`
  (params (ActionValue :type Boolean) (ElapsedSeconds :type "Float (double-precision)") (TriggeredSeconds :type "Float (double-precision)") (InputAction :type "InputAction Object Reference" :default "/Game/Inputs/Run.Run"))
  (bind _charactermovement (`self.CharacterMovement`))
  ;[0.08209 0.5758 1] Movement
  (:`Started`
    (set `CharacterMovementComponent.MaxWalkSpeed` 1200.0 _charactermovement))
  (:`Completed`
    (set `CharacterMovementComponent.MaxWalkSpeed` 600.0 _charactermovement)))

(fn `UserConstructionScript`)